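; First-person player Blueprint that handles looking, jumping and four-direction movement through Enhanced Input.
; BeginPlay adds the FP_IMC mapping context; Look drives controller yaw and pitch, and Jump starts and stops jumping.
; Opposing move actions share one AddMovementInput per axis along the actor's forward or right vector, scaled by subtracted action values.
; Move actions also set and clear LeftValue or RightValue, which this graph never reads.
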(event Input|EnhancedActionEvents|EnhancedInputActionLook_IA
  (params (ActionValue :type Vector%202D%20Structure) (ElapsedSeconds :type Float%20%28double-precision%29) (TriggeredSeconds :type Float%20%28double-precision%29) (InputAction :type Input%20Action%20Object%20Reference :default "/Game/Inputs/InputActions/Look_IA.Look_IA"))
  ;[0.15 0.15 0.15 0.5] Look_IA
  (:Triggered
    (Pawn|Input|AddControllerYawInput (.x ActionValue))
    (Pawn|Input|AddControllerPitchInput (.y ActionValue))))

(event Input|EnhancedActionEvents|EnhancedInputActionJump_IA
  (params (ActionValue :type Vector%202D%20Structure) (ElapsedSeconds :type Float%20%28double-precision%29) (TriggeredSeconds :type Float%20%28double-precision%29) (InputAction :type Input%20Action%20Object%20Reference :default "/Game/Inputs/InputActions/Jump_IA.Jump_IA"))
  ;[0.15 0.15 0.15 0.5] Jump_IA
  (:Triggered
    (Character|Jump))
  (:Completed
    (Character|StopJumping)))

(event Input|EnhancedActionEvents|EnhancedInputActionForward_IA
  (params (ActionValue :type Float%20%28double-precision%29) (ElapsedSeconds :type Float%20%28double-precision%29) (TriggeredSeconds :type Float%20%28double-precision%29) (InputAction :type Input%20Action%20Object%20Reference :default "/Game/Inputs/InputActions/Forward_IA.Forward_IA"))
  ;[0.15 0.15 0.15 0.5] Movement
  (:Triggered
    (Variables|Default|SetLeftValue 1.0)
    (Pawn|Input|AddMovementInput (Transformation|GetActorForwardVector) (- ActionValue (stale Input|EnhancedActionEvents|EnhancedInputActionBackward_IA ActionValue)) false))
  (:Canceled
    (Variables|Default|SetLeftValue 0.0 :!label _label))
  (:Completed
    (goto _label)))

(event Input|EnhancedActionEvents|EnhancedInputActionLeft_IA
  (params (ActionValue :type Float%20%28double-precision%29) (ElapsedSeconds :type Float%20%28double-precision%29) (TriggeredSeconds :type Float%20%28double-precision%29) (InputAction :type Input%20Action%20Object%20Reference :default "/Game/Inputs/InputActions/Left_IA.Left_IA"))
  ;[0.15 0.15 0.15 0.5] Movement
  (:Triggered
    (Variables|Default|SetLeftValue 1.0)
    (Pawn|Input|AddMovementInput (Transformation|GetActorRightVector) (* (- ActionValue (stale Input|EnhancedActionEvents|EnhancedInputActionRight_IA ActionValue)) -1.0) false))
  (:Canceled
    (Variables|Default|SetLeftValue 0.0 :!label _label))
  (:Completed
    (goto _label)))

(event Input|EnhancedActionEvents|EnhancedInputActionRight_IA
  (params (ActionValue :type Float%20%28double-precision%29) (ElapsedSeconds :type Float%20%28double-precision%29) (TriggeredSeconds :type Float%20%28double-precision%29) (InputAction :type Input%20Action%20Object%20Reference :default "/Game/Inputs/InputActions/Right_IA.Right_IA"))
  ;[0.15 0.15 0.15 0.5] Movement
  (:Triggered
    (Variables|Default|SetRightValue 1.0)
    (Pawn|Input|AddMovementInput (Transformation|GetActorRightVector) (* (- (stale Input|EnhancedActionEvents|EnhancedInputActionLeft_IA ActionValue) ActionValue) -1.0) false))
  (:Canceled
    (Variables|Default|SetRightValue 0.0 :!label _label))
  (:Completed
    (goto _label)))

(event Input|EnhancedActionEvents|EnhancedInputActionBackward_IA
  (params (ActionValue :type Float%20%28double-precision%29) (ElapsedSeconds :type Float%20%28double-precision%29) (TriggeredSeconds :type Float%20%28double-precision%29) (InputAction :type Input%20Action%20Object%20Reference :default "/Game/Inputs/InputActions/Backward_IA.Backward_IA"))
  ;[0.15 0.15 0.15 0.5] Movement
  (:Triggered
    (Variables|Default|SetRightValue 1.0)
    (Pawn|Input|AddMovementInput (Transformation|GetActorForwardVector) (- (stale Input|EnhancedActionEvents|EnhancedInputActionForward_IA ActionValue) ActionValue) false))
  (:Canceled
    (Variables|Default|SetRightValue 0.0 :!label _label))
  (:Completed
    (goto _label)))

(event EventBeginPlay
  ;[0.15 0.15 0.15 0.5] Input Mapping Context
  (bind _asplayer_controller (Utilities|Casting|CastToPlayerController (Pawn|GetController)))
  (Utilities|IsValid (PlayerController|LocalPlayerSubsystems|GetEnhancedInputLocalPlayerSubsystem _asplayer_controller)
    (:Is%20Valid
      (Input|AddMappingContext (PlayerController|LocalPlayerSubsystems|GetEnhancedInputLocalPlayerSubsystem _asplayer_controller) "/Game/Inputs/FP_IMC.FP_IMC" 0 "(bIgnoreAllPressedKeysUntilRelease=True,bForceImmediately=False,bNotifyUserSettings=False)"))))

(fn ConstructionScript)